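; BP_note is a rhythm note actor that travels along the first lane spline of the BP_spline actor in the level.
; On BeginPlay it finds that actor, looks up its cue name in a map to set the sphere's material, and prints the result.
; MoveNotes plays a timeline at a rate of one over the spline actor's TimeToComplete, lerping distance along Lane01 to update position and rotation.
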(event `self.ReceiveBeginPlay`
  (bind _returnvalue (`GameplayStatics.GetActorOfClass` "/Game/Base_Damien/Music_tools/BP_spline.BP_spline_C"))
  (set `self.RythmeSpline` _returnvalue)
  (bind _value (`BlueprintMapLibrary.Map_Find` (`self.DicoCueToSprite`) (`/Game/Base_Damien/Music_tools/BP_spline.CueName` _returnvalue)))
  (`KismetSystemLibrary.PrintString` (`KismetSystemLibrary.GetDisplayName` _value))
  (`PrimitiveComponent.SetMaterial` (`self.Sphere`) 0 _value))

(event `MoveNotes`
  (bind _lane_01 (`/Game/Base_Damien/Music_tools/BP_spline.Lane_01` (`self.RythmeSpline`)))
  (`TimelineComponent.SetPlayRate` (`self.Timeline`) (/ 1.0 (`/Game/Base_Damien/Music_tools/BP_spline.TimeToComplete` (stale `self.ReceiveBeginPlay` _returnvalue))))
  (bind (_direction _newtrack_0) (`Timeline|Timeline`)
    (:`Update`
      (bind _returnvalue (`KismetMathLibrary.Lerp` 0.0 (`SplineComponent.GetSplineLength` (`/Game/Base_Damien/Music_tools/BP_spline.Lane_01` (`self.RythmeSpline`))) _newtrack_0))
      (`self.K2_SetActorTransform` (`KismetMathLibrary.MakeTransform` (`SplineComponent.GetLocationAtDistanceAlongSpline` _lane_01 _returnvalue "World") (`SplineComponent.GetRotationAtDistanceAlongSpline` _lane_01 _returnvalue "World") (`SceneComponent.RelativeScale3D` (`self.Sphere`)))))))

(fn `UserConstructionScript`)