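; BP_verification is an actor that checks whether the player's key matches the expected one for a dance step.
; On BeginPlay it caches references to BP_dancing_manager and the BONHOMME actor.
; The verifie event looks up the passed index in the Verif map, compares it with BONHOMME's Key and prints success or failure as debug text.
; A HUD_damien lookup is present but never runs.
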(event `verifie`
  (params (NewParam :type Integer))
  (bind _value (`BlueprintMapLibrary.Map_Find` (`self.verif`) NewParam))
  (`KismetSystemLibrary.PrintString` (`KismetStringLibrary.Concat_StrStr` "index :  " (`KismetStringLibrary.Conv_IntToString` NewParam) "  key : " (`/Game/Base_Damien/Characters/Principal/Anim/BONHOMME.key` (stale `self.ReceiveBeginPlay` _asbonhomme)) "  verif : " _value))
  (if (`KismetStringLibrary.EqualEqual_StrStr` _value (stale `self.ReceiveBeginPlay` _output_get))
    (`KismetSystemLibrary.PrintString` "BRAVO")
    (else
      (`KismetSystemLibrary.PrintString` "NOOON"))))

(event `self.ReceiveBeginPlay`
  (bind _returnvalue (`GameplayStatics.GetActorOfClass` "/Game/Base_Damien/Dance_tools/BP_dancing_manager.BP_dancing_manager_C"))
  (bind _asbp_dancing_manager (cast `/Game/Base_Damien/Dance_tools/BP_dancing_manager` _returnvalue))
  (set `/Game/Base_Damien/Dance_tools/BP_dancing_manager.index` (`/Game/Base_Damien/Dance_tools/BP_dancing_manager.index` _asbp_dancing_manager) _asbp_dancing_manager)
  (bind _returnvalue_2 (`GameplayStatics.GetActorOfClass` "/Game/Base_Damien/Characters/Principal/Anim/BONHOMME.BONHOMME_C"))
  (bind _asbonhomme (cast `/Game/Base_Damien/Characters/Principal/Anim/BONHOMME` _returnvalue_2))
  (bind _output_get (set `/Game/Base_Damien/Characters/Principal/Anim/BONHOMME.key` (`/Game/Base_Damien/Characters/Principal/Anim/BONHOMME.key` _asbonhomme) _asbonhomme)))

(event `self.ReceiveTick`
  (params (DeltaSeconds :type "Float (single-precision)")))

(fn `UserConstructionScript`)