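; BP_dancing_manager is the manager for the dance tools, relaying dance inputs by index to the HUD and a verification actor.
; On BeginPlay it caches the player's HUD_damien and the BP_verification actor found in the level.
; Its dance event stores the incoming index, triggers the HUD widget with it, then passes it to BP_verification to be checked.
; A debug print of the index is left disconnected.
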(event `self.ReceiveBeginPlay`
  (bind _asnew_hud (cast `/Game/Dance_game/suite/UI/HUD_damien` (`PlayerController.GetHUD` (`GameplayStatics.GetPlayerController` 0))))
  (set `self.MyHUD` _asnew_hud)
  (bind _returnvalue (`GameplayStatics.GetActorOfClass` "/Game/Base_Damien/Dance_tools/BP_verification.BP_verification_C"))
  (bind _asbp_verification (cast `/Game/Base_Damien/Dance_tools/BP_verification` _returnvalue)))

(event `dance`
  (params (index :type Integer))
  (bind _output_get (set `self.index` index))
  (`/Game/Dance_game/suite/UI/UI_interface.TRIG` (`/Game/Dance_game/suite/UI/HUD_damien.NewVar` (`self.MyHUD`)) _output_get)
  (`/Game/Base_Damien/Dance_tools/BP_verification.verifie` (stale `self.ReceiveBeginPlay` _asbp_verification) _output_get))

(fn `UserConstructionScript`)