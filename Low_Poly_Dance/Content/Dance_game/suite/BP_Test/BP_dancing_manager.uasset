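; Manager actor that relays dance step events, by index, to the HUD and to a second actor.
; On BeginPlay it caches the player's NewHUD and a cast reference to an actor found by class lookup.
; The dance event triggers the HUD's NewVar with the index, then calls Verifie on that actor with the same index.
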(event `self.ReceiveBeginPlay`
  (bind _asnew_hud (cast `/Game/Dance_game/suite/UI/NewHUD` (`PlayerController.GetHUD` (`GameplayStatics.GetPlayerController` 0))))
  (set `self.MyHUD` _asnew_hud)
  (bind _returnvalue (`GameplayStatics.GetActorOfClass` null))
  (bind _asbp_verification (cast `` _returnvalue)))

(event `dance`
  (params (index :type Integer))
  (bind _output_get (set `self.index` index))
  (`/Game/Dance_game/suite/UI/UI_interface.TRIG` (`/Game/Dance_game/suite/UI/NewHUD.NewVar` (`self.MyHUD`)) _output_get)
  (`self.verifie` (stale `self.ReceiveBeginPlay` _asbp_verification) _output_get))

(fn `UserConstructionScript`)